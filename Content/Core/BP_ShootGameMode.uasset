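; BP_ShootGameMode is the game mode for a shooting game, managing the HUD and the end-of-game screen.
; On BeginPlay it binds the game-finished event, adds the HUD and a collapsed W_GameFinished widget to the viewport, and sets game-only input with the cursor hidden.
; When the game finishes, it reveals that pre-created widget, switches to UI-only input and shows the mouse cursor.
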(event `self.ReceiveBeginPlay`
  (add `self.OnGameFinished` (`|CreateDelegate` :!event `OnGameFinished_Event`))
  (`self.NewFunction_0`))

(event `OnGameFinished_Event`
  (bind _returnvalue (`GameplayStatics.GetPlayerController` 0))
  (`Widget.SetVisibility` (`self.W_GameFinished`) "Visible")
  (`WidgetBlueprintLibrary.SetInputMode_UIOnlyEx` _returnvalue null)
  (set `PlayerController.bShowMouseCursor` true _returnvalue))

(fn `NewFunction_0`
  (bind _returnvalue (`GameplayStatics.GetPlayerController` 0))
  (bind _returnvalue_2 (`|CreateWidget` "/Game/UI/W_HUD.W_HUD_C"))
  (`UserWidget.AddToViewport` _returnvalue_2 0)
  (`WidgetBlueprintLibrary.SetInputMode_GameOnly` _returnvalue)
  (set `PlayerController.bShowMouseCursor` false _returnvalue)
  (bind _returnvalue_3 (`|CreateWidget` "/Game/UI/W_GameFinished.W_GameFinished_C"))
  (bind _output_get (set `self.W_GameFinished` _returnvalue_3))
  (`UserWidget.AddToViewport` _output_get 0)
  (`Widget.SetVisibility` (`self.W_GameFinished`) "Collapsed"))

(fn `UserConstructionScript`)