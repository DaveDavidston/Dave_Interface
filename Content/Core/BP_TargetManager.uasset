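; Target manager actor for the shooting game mode that spawns shootable targets one at a time and signals when the game finishes.
; On BeginPlay it builds a shuffle bag of target indices from the game mode's class list and per-target count, then spawns the first.
; Each shot event spawns a random remaining target at a random yaw around a pivot, facing the manager, or calls game finished when none remain.
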(event `self.ReceiveBeginPlay`
  (`self.InitTargetsToSpawn`)
  (bind _asbp_shoot_game_mode (cast `/Game/Core/BP_ShootGameMode` (`GameplayStatics.GetGameMode`)))
  (add `/Game/Core/BP_ShootGameMode.OnTargetShot` _asbp_shoot_game_mode (`|CreateDelegate` :!event `OnTargetShot_Event`))
  (`self.SpawnTarget`))

(event `OnTargetShot_Event`
  (bind _targetavailable (`self.SpawnTarget`))
  (if (not _targetavailable)
    (bind _asbp_shoot_game_mode (cast `/Game/Core/BP_ShootGameMode` (`GameplayStatics.GetGameMode`)))
    (`/Game/Core/BP_ShootGameMode.OnGameFinished` _asbp_shoot_game_mode)))

(fn `GetNextTargetClass`
  (returns (TargetClass :type "Target Class Reference") (TargetAvailable :type Boolean))
  (locals (ReturnTargetClass :type "Target Class Reference") (RandomIndex :type Integer :default 0) (NewLocalVar_0 :type Integer))
  (if (`KismetArrayLibrary.Array_IsEmpty` (`self.TargetsToSpawn`))
    (return null false)
    (else
      (bind _output_get (set `local.RandomIndex` (`.OutIndex` (`KismetArrayLibrary.Array_Random` (`self.TargetsToSpawn`)))))
      (bind _asbp_shoot_game_mode (cast `/Game/Core/BP_ShootGameMode` (`GameplayStatics.GetGameMode`)))
      (set `local.ReturnTargetClass` (`|GetArrayItem` (`/Game/Core/BP_ShootGameMode.Targets` _asbp_shoot_game_mode) (`|GetArrayItem` (`self.TargetsToSpawn`) _output_get)))
      (`KismetArrayLibrary.Array_Remove` (`self.TargetsToSpawn`) _output_get)
      (return (`local.ReturnTargetClass`) true))))

(fn `GetRandomSpawnTransform`
  (returns (SpawnTransform :type "Transform Structure"))
  (locals (RandomRot :type "Float (double-precision)" :default 0.0))
  (bind _returnvalue (`KismetMathLibrary.RandomFloatInRange` -150.0 -30.0))
  (set `local.RandomRot` _returnvalue)
  (`SceneComponent.K2_SetRelativeRotation` (`self.Middle`) (`KismetMathLibrary.MakeRotator` 0.0 0.0 _returnvalue) false false)
  (return (`KismetMathLibrary.MakeTransform` (`SceneComponent.K2_GetComponentLocation` (`self.Out`)) (`KismetMathLibrary.FindLookAtRotation` (`SceneComponent.K2_GetComponentLocation` (`self.Out`)) (`self.K2_GetActorLocation`)) (2.0 2.0 2.0))))

(fn `InitTargetsToSpawn`
  (bind _asbp_shoot_game_mode (cast `/Game/Core/BP_ShootGameMode` (`GameplayStatics.GetGameMode`)))
  (for _index (range (`KismetArrayLibrary.Array_Length` (`/Game/Core/BP_ShootGameMode.Targets` _asbp_shoot_game_mode)))
    (for _ (range 1 (+ (`/Game/Core/BP_ShootGameMode.NumInstancesPerTarget` _asbp_shoot_game_mode) 1))
      (`KismetArrayLibrary.Array_Add` (`self.TargetsToSpawn`) _index))))

(fn `SpawnTarget`
  (returns (TargetAvailable :type Boolean))
  (bind (_targetclass _targetavailable) (`self.GetNextTargetClass`))
  (if _targetavailable
    (bind _returnvalue (`|SpawnActorFromClass` _targetclass (`self.GetRandomSpawnTransform`) "Undefined" "OverrideRootScale" null null))
    (bind _asbp_shoot_game_mode (cast `/Game/Core/BP_ShootGameMode` (`GameplayStatics.GetGameMode`)))
    (`/Game/Core/BP_ShootGameMode.OnTargetSpawned` _asbp_shoot_game_mode _returnvalue))
  (return _targetavailable))

(fn `UserConstructionScript`)