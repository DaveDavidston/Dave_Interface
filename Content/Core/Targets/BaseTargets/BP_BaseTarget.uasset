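; BP_BaseTarget is the base Blueprint for shootable targets, reporting hits to the game mode.
; On BeginPlay it records its spawn time, caches the player's BP_ShootingCharacter and stores the initial distance between that character's camera and its own mesh.
; HitbyItem calls CallOnTargetShot on BP_ShootGameMode, while helper functions return time elapsed since spawn and current distance to the player.
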(event `self.ReceiveBeginPlay`
  (set `self.SpawnTime` (`KismetSystemLibrary.GetGameTimeInSeconds`))
  (bind _asbp_character (cast `/Game/Core/BP_ShootingCharacter` (`GameplayStatics.GetPlayerPawn` 0)))
  (set `self.Character` _asbp_character)
  (set `self.InitialDistance` (`self.GetDistanceToPlayer`)))

(event `self.HitByItem`
  (bind _asbp_shoot_game_mode (cast `/Game/Core/BP_ShootGameMode` (`GameplayStatics.GetGameMode`)))
  (`/Game/Core/BP_ShootGameMode.OnTargetShot` _asbp_shoot_game_mode))

(fn `GetDistanceToPlayer`
  (returns (Distance :type "Float (double-precision)"))
  (return (`KismetMathLibrary.Vector_Distance` (`SceneComponent.K2_GetComponentLocation` (`/Game/Core/BP_ShootingCharacter.Camera` (`self.Character`))) (`SceneComponent.K2_GetComponentLocation` (`self.Mesh`)))))

(fn `GetElapsedTime`
  (returns (ElaspedTime :type "Float (double-precision)"))
  (return (- (`KismetSystemLibrary.GetGameTimeInSeconds`) (`self.SpawnTime`))))

(fn `UserConstructionScript`)